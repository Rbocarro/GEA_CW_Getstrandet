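; Sliding door actor that opens when the correct code is entered on its in-world keypad widget.
; BeginPlay binds to the Keypad_UI code-entered event, and CheckCode compares the entry with CorrectCode, clears it, recolors the text and plays success or error audio.
; A match sets UnlockDoor, which Tick polls to play, after a delay and only once, the door sound and a timeline that slides the mesh.
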(event `self.ReceiveTick`
  (params (DeltaSeconds :type "Float (single-precision)"))
  (if (`self.UnlockDoor`)
    (`KismetSystemLibrary.Delay` (`self.Doordelay`))
    (`/Engine/EditorBlueprintResources/StandardMacros.DoOnce` false
      (:`Completed`
        (`GameplayStatics.PlaySound2D` "/Game/Sound/Interface_And_Item_Sounds/Spaceship_Door_Sound1.Spaceship_Door_Sound1" 1.0 0.5 0.0 null null)
        (bind (_direction _slide) (`Timeline|Timeline_0`)
          (:`Update`
            (`SceneComponent.K2_SetRelativeLocation` (`self.SM_Scifi_Door_01_Door`) _slide false false)))))))

(event `self.ReceiveBeginPlay`
  (set `self.UnlockDoor` false)
  (bind _askeypad_ui (cast `/Game/UI/Keypad_UI` (`WidgetComponent.GetUserWidgetObject` (`self.KeypadWidget`))))
  (bind _output_get (set `self.Keypad UI` _askeypad_ui))
  (add `/Game/UI/Keypad_UI.CodeEntered` _output_get (`|CreateDelegate` :!event `CheckCode`)))

(fn `CheckCode`
  (params (CodeEntered :type String) (KeypadUI :type "/Game/UI/Keypad_UI Object Reference"))
  (locals (NewLocalVar_0 :type "SlateColor Structure" :default (struct :`SpecifiedColor` (struct :`R` 1.0 :`G` 1.0 :`B` 1.0 :`A` 1.0) :`ColorUseRule` "UseColor_Specified")))
  (bind _keypad_ui (`self.Keypad UI`))
  (bind _keypad_ui_2 (`self.Keypad UI`))
  (if (`KismetStringLibrary.EqualEqual_StrStr` CodeEntered (`self.CorrectCode`))
    (set `/Game/UI/Keypad_UI.CurrentCode` "" _keypad_ui)
    (`TextBlock.SetColorAndOpacity` (`/Game/UI/Keypad_UI.CodeText` _keypad_ui) (`self.In Color and Opacity`))
    (`GameplayStatics.PlaySound2D` "/Game/Sound/Interface_And_Item_Sounds/Cues/Coins_10_Cue.Coins_10_Cue" 1.0 1.0 0.0 null null)
    (set `self.UnlockDoor` true)
    (else
      (set `/Game/UI/Keypad_UI.CurrentCode` "" _keypad_ui_2)
      (`TextBlock.SetColorAndOpacity` (`/Game/UI/Keypad_UI.CodeText` _keypad_ui_2) (`self.In Color and Opacity_2`))
      (`GameplayStatics.PlaySound2D` "/Game/Sound/Interface_And_Item_Sounds/WAV/Error_Buzz_05.Error_Buzz_05" 0.5 1.0 0.0 null null))))

(fn `UserConstructionScript`)